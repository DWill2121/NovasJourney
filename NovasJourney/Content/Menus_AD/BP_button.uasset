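; BP_button is a menu button that keeps mouse hover and keyboard focus in sync and restyles itself to show which state it is in.
; Start and Begin each set a fast looping timer by function name, polling CheckState and CheckFocus respectively, which contain identical logic.
; Hover takes keyboard focus and applies MouseStyle; otherwise the style is Selected or NotSelected, depending on focus.
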(fn Start
  (Utilities|Time|SetTimerbyFunctionName 0 "CheckState" 0.01 true))

(fn CheckState
  (if (Widget|IsHovered)
    (Widget|SetKeyboardFocus)
    (Class|Button|SetStyle (Variables|Default|GetMouseStyle))
    (else
      (Class|Button|SetStyle (select (Class|Widget|HasKeyboardFocus) (Variables|Default|GetSelected) (Variables|Default|GetNotSelected))))))

(fn Begin
  (Utilities|Time|SetTimerbyFunctionName 0 "CheckFocus" 0.01 true))

(fn CheckFocus
  (if (Widget|IsHovered)
    (Widget|SetKeyboardFocus)
    (Class|Button|SetStyle (Variables|Default|GetMouseStyle))
    (else
      (Class|Button|SetStyle (select (Class|Widget|HasKeyboardFocus) (Variables|Default|GetSelected) (Variables|Default|GetNotSelected))))))