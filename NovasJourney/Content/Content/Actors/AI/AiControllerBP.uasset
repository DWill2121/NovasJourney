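; AI controller that runs the AITree behavior tree on possessed enemies and feeds perception results into its blackboard.
; Perception updates on a Nova2 actor set CanSeePlayer from whether the stimulus was sensed.
; A CompleteSenses function, not called in these graphs, maps senses by array index to CanSeePlayer or to IsInvestigating and TargetLocation.
; Its second sense also plays a sound at the receiver's location.
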(event OnTargetPerceptionUpdated(AIPerception)
  (params (Actor :type Actor%20Object%20Reference) (Stimulus :type AI%20Stimulus%20Structure))
  (Utilities|Casting|CastToNova2 Actor)
  (bind _output_get (Variables|Default|SetCanSeePlayer (.bsuccessfullysensed Stimulus)))
  (AI|Components|Blackboard|SetValueasBool (AI|GetBlackboard 0) (Utilities|Name|MakeLiteralName "CanSeePlayer") _output_get))

(event EventBeginPlay
  (AI|RunBehaviorTree "/Game/Content/Actors/AI/AITree.AITree")
  (bind _asbasic_ai (Utilities|Casting|CastToBasicAI (Pawn|GetControlledPawn)))
  (Variables|Default|SetAi _asbasic_ai))

(fn ConstructionScript)

(fn CompleteSenses
  (params (Array :type Array%20of%20AI%20Stimulus%20Structures))
  (for (_array_element _array_index) Array
    (LocalVariables|SetLocal_Sense _array_element)
    (switch int _array_index
      (:0
        (AI|Components|Blackboard|SetValueasBool (AI|GetBlackboard 0) (Utilities|Name|MakeLiteralName "CanSeePlayer") (.bsuccessfullysensed (LocalVariables|GetLocal_Sense))))
      (:1
        (if (.bsuccessfullysensed (LocalVariables|GetLocal_Sense))
          (Audio|PlaySoundatLocation 0 (.receiverlocation (LocalVariables|GetLocal_Sense)) "0, 0, 0" 1.0 1.0 0.0 0 0 0)
          (AI|Components|Blackboard|SetValueasBool (AI|GetBlackboard 0) (Utilities|Name|MakeLiteralName "IsInvestigating") (.bsuccessfullysensed (LocalVariables|GetLocal_Sense)) :!label _label)
          (AI|Components|Blackboard|SetValueasVector (AI|GetBlackboard 0) (Utilities|Name|MakeLiteralName "TargetLocation") (.stimuluslocation (LocalVariables|GetLocal_Sense)))))
      (:2
        (if (.bsuccessfullysensed (LocalVariables|GetLocal_Sense))
          (goto _label))))))