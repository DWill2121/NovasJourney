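; BP_Checkpoint is a checkpoint actor that updates the player's respawn location.
; When a Nova2 overlaps its Trigger, it writes the checkpoint actor's own location into that character's SpawnPoint.
; An unconnected chain that would print a message and save the player's location to the "check" save slot never runs, so the checkpoint itself saves nothing to disk.
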(event OnComponentBeginOverlap(Trigger)
  (params (OverlappedComponent :type Primitive%20Component%20Object%20Reference) (OtherActor :type Actor%20Object%20Reference) (OtherComp :type Primitive%20Component%20Object%20Reference) (OtherBodyIndex :type Integer) (bFromSweep :type Boolean) (SweepResult :type Hit%20Result%20Structure%20%28by%20ref%29))
  (bind _asnova_2 (Utilities|Casting|CastToNova2 OtherActor))
  (bind _output_get (Variables|Default|SetPlayerLoc2 (Transformation|GetActorLocation)))
  (Variables|/Game/Content/Actors/Character/Nova2.Nova2_C|SetSpawnPoint _asnova_2 _output_get))

(event EventBeginPlay)

(event Collision|EventActorBeginOverlap
  (params (OtherActor :type Actor%20Object%20Reference)))

(event EventTick
  (params (DeltaSeconds :type Float%20%28single-precision%29)))

(fn ConstructionScript)