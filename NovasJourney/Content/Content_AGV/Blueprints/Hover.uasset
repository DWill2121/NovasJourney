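; Hover is a component in the AGV content that makes its owning actor float above surfaces using physics.
; On BeginPlay it finds the owner's primitive component and turns on physics simulation.
; Each tick it traces straight down on the Visibility channel and, on a hit, pushes that body along the surface normal with a force that fades linearly to zero at the trace length.
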(event EventBeginPlay
  (bind _output_get (Variables|Default|SetPrimitive_Component (Utilities|Array|Get(acopy) (Utilities|Array|MakeArray (Actor|GetComponentbyClass (Components|GetOwner) "/Script/Engine.PrimitiveComponent")))))
  (Physics|SetSimulatePhysics _output_get true))

(event EventTick
  (params (DeltaSeconds :type Float%20%28single-precision%29))
  (bind _returnvalue (Transformation|GetWorldLocation))
  (bind (_outhit _returnvalue_2) (Collision|LineTraceByChannel _returnvalue (- _returnvalue (Math|Vector|MakeVector 0.0 0.0 (Variables|Default|GetTrace_Length))) "TraceTypeQuery1" false 0 "None"))
  (if _returnvalue_2
    (Physics|AddForce (Variables|Default|GetPrimitive_Component) (* (.ImpactNormal (Collision|BreakHitResult _outhit)) (Math|Float|Lerp 5e+06 0.0 (/ (Math|Vector|VectorLength (- (.Location (Collision|BreakHitResult _outhit)) (Transformation|GetWorldLocation))) (Variables|Default|GetTrace_Length)))) "None" false)))