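; Dialogue_Box_No_Halt is an overlap-triggered actor that shows a dialogue box on screen without pausing the game or player.
; The first overlap by any actor creates a Dialogue_Box_WIDG for player 0, fills it with MyTextForEngine and shows it.
; End overlap reapplies the text and hides both the widget and its inner DialogueBoxAGV element.
; A DoOnce with no reset means the dialogue appears only once per instance.
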(event Collision|EventActorBeginOverlap
  (params (OtherActor :type Actor%20Object%20Reference))
  (Utilities|FlowControl|DoOnce false
    (:Completed
      (bind _returnvalue (UserInterface|CreateWidget "/Game/Content_AGV/UI/Dialogue_Box_WIDG.Dialogue_Box_WIDG_C" (Game|GetPlayerController 0)))
      (UserInterface|Viewport|AddtoViewport _returnvalue 0)
      (Variables|/Game/Content_AGV/UI/Dialogue_Box_WIDG.Dialogue_Box_WIDG_C|SetMy_Text _returnvalue (Variables|Default|GetMy_Text_For_Engine))
      (Widget|SetVisibility _returnvalue "Visible"))))

(event Collision|EventActorEndOverlap
  (params (OtherActor :type Actor%20Object%20Reference))
  (Variables|/Game/Content_AGV/UI/Dialogue_Box_WIDG.Dialogue_Box_WIDG_C|SetMy_Text (stale Collision|EventActorBeginOverlap _returnvalue) (Variables|Default|GetMy_Text_For_Engine))
  (Widget|SetVisibility (stale Collision|EventActorBeginOverlap _returnvalue) "Hidden")
  (Widget|SetVisibility (Variables|/Game/Content_AGV/UI/Dialogue_Box_WIDG.Dialogue_Box_WIDG_C|GetDialogue_Box_AGV (stale Collision|EventActorBeginOverlap _returnvalue)) "Hidden"))

(fn ConstructionScript)