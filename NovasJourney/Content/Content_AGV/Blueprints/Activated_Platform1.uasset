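; Spline-following platform that sets off when the Nova1 actor enters its trigger box.
; After a short delay, the MovePlatform timeline drives PlatformBase along the spline at a set rate, matching the spline's yaw.
; Leaving the box reverses the timeline after a delay.
; A never-reset DoOnce precedes the cast, so only the first overlap by any actor can start forward travel.
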(event OnComponentBeginOverlap(Box)
  (params (OverlappedComponent :type Primitive%20Component%20Object%20Reference) (OtherActor :type Actor%20Object%20Reference) (OtherComp :type Primitive%20Component%20Object%20Reference) (OtherBodyIndex :type Integer) (bFromSweep :type Boolean) (SweepResult :type Hit%20Result%20Structure%20%28by%20ref%29))
  (bind _spline (Variables|Default|GetSpline))
  (Utilities|FlowControl|DoOnce false
    (:Completed
      (Utilities|Casting|CastToNova1 OtherActor)
      (Utilities|FlowControl|Delay 1.0)
      (Components|Timeline|SetPlayRate (Variables|Default|GetMovePlatform) (Variables|Default|GetRate))
      (bind _traveldistance (Timeline|MovePlatform Play)
        (:Update
          (Transformation|SetWorldLocation (Variables|Default|GetPlatform_Base) (Spline|GetLocationatDistanceAlongSpline _spline (* _traveldistance (Spline|GetSplineLength (Variables|Default|GetSpline))) "World") false false)
          (Transformation|SetRelativeRotation (Variables|Default|GetPlatform_Base) (Math|Rotator|MakeRotator 0.0 0.0 (.yaw (Spline|GetRotationatDistanceAlongSpline _spline (* _traveldistance (Spline|GetSplineLength (Variables|Default|GetSpline))) "Local"))) false false))))))

(event OnComponentEndOverlap(Box)
  (params (OverlappedComponent :type Primitive%20Component%20Object%20Reference) (OtherActor :type Actor%20Object%20Reference) (OtherComp :type Primitive%20Component%20Object%20Reference) (OtherBodyIndex :type Integer))
  (bind _spline (Variables|Default|GetSpline))
  (Utilities|Casting|CastToNova1 OtherActor)
  (Utilities|FlowControl|Delay 2.0)
  (bind _traveldistance (Timeline|MovePlatform Reverse)
    (:Update
      (Transformation|SetWorldLocation (Variables|Default|GetPlatform_Base) (Spline|GetLocationatDistanceAlongSpline _spline (* _traveldistance (Spline|GetSplineLength (Variables|Default|GetSpline))) "World") false false)
      (Transformation|SetRelativeRotation (Variables|Default|GetPlatform_Base) (Math|Rotator|MakeRotator 0.0 0.0 (.yaw (Spline|GetRotationatDistanceAlongSpline _spline (* _traveldistance (Spline|GetSplineLength (Variables|Default|GetSpline))) "Local"))) false false))))

(event Collision|EventActorBeginOverlap
  (params (OtherActor :type Actor%20Object%20Reference)))

(event EventTick
  (params (DeltaSeconds :type Float%20%28single-precision%29)))

(event EventBeginPlay
  (bind _spline (Variables|Default|GetSpline))
  (bind _returnvalue (Spline|GetRotationatDistanceAlongSpline _spline 0.0 "Local"))
  (Transformation|SetRelativeRotation (Variables|Default|GetPlatform_Base) (Math|Rotator|MakeRotator (.roll _returnvalue) 0.0 (.yaw _returnvalue)) false false))

(fn ConstructionScript)