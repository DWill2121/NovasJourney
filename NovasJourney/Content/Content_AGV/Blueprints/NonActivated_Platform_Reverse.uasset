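; Moving platform actor that starts travelling along its spline on BeginPlay, with no activation needed.
; A timeline, with play rate set by Rate, maps TravelDistance onto spline length to place PlatformBase in world space.
; Each update also applies the spline's local yaw as relative rotation, keeping pitch and roll level.
; When the timeline finishes, the Reverse event plays it backwards.
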(event Custom|Reverse
  (bind _spline (Variables|Default|GetSpline))
  (bind _traveldistance (Timeline|MovePlatform Reverse)
    (:Update
      (Transformation|SetWorldLocation (Variables|Default|GetPlatform_Base) (Spline|GetLocationatDistanceAlongSpline _spline (* _traveldistance (Spline|GetSplineLength (Variables|Default|GetSpline))) "World") false false)
      (Transformation|SetRelativeRotation (Variables|Default|GetPlatform_Base) (Math|Rotator|MakeRotator 0.0 0.0 (.yaw (Spline|GetRotationatDistanceAlongSpline _spline (* _traveldistance (Spline|GetSplineLength (Variables|Default|GetSpline))) "Local"))) false false))
    (:Finished
      (CallFunction|Reverse))))

(event Collision|EventActorBeginOverlap
  (params (OtherActor :type Actor%20Object%20Reference)))

(event EventTick
  (params (DeltaSeconds :type Float%20%28single-precision%29)))

(event EventBeginPlay
  (bind _spline (Variables|Default|GetSpline))
  (Components|Timeline|SetPlayRate (Variables|Default|GetMovePlatform) (Variables|Default|GetRate))
  (bind _traveldistance (Timeline|MovePlatform Play)
    (:Update
      (Transformation|SetWorldLocation (Variables|Default|GetPlatform_Base) (Spline|GetLocationatDistanceAlongSpline _spline (* _traveldistance (Spline|GetSplineLength (Variables|Default|GetSpline))) "World") false false)
      (Transformation|SetRelativeRotation (Variables|Default|GetPlatform_Base) (Math|Rotator|MakeRotator 0.0 0.0 (.yaw (Spline|GetRotationatDistanceAlongSpline _spline (* _traveldistance (Spline|GetSplineLength (Variables|Default|GetSpline))) "Local"))) false false))
    (:Finished
      (CallFunction|Reverse))))

(fn ConstructionScript)