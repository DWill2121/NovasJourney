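; Dialogue_Box is an overlap-triggered dialogue actor that shows a Dialogue_Box_WIDG displaying its MyTextForEngine text.
; The first overlap, gated by DoOnce, creates the widget, shakes the camera, disables player input, toggles the TextRender's visibility and restores input after a short delay.
; Every end overlap hides the widget and, after a delay, rejoins that sequence at the TextRender toggle and delayed input restore.
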(event Collision|EventActorBeginOverlap
  (params (OtherActor :type Actor%20Object%20Reference))
  (bind _returnvalue (Game|GetPlayerCharacter 0))
  (bind _returnvalue_2 (Game|GetPlayerController 0))
  (Utilities|FlowControl|DoOnce false
    (:Completed
      (bind _returnvalue_3 (UserInterface|CreateWidget "/Game/Content_AGV/UI/Dialogue_Box_WIDG.Dialogue_Box_WIDG_C" (Game|GetPlayerController 0)))
      (UserInterface|Viewport|AddtoViewport _returnvalue_3 0)
      (Variables|/Game/Content_AGV/UI/Dialogue_Box_WIDG.Dialogue_Box_WIDG_C|SetMy_Text _returnvalue_3 (Variables|Default|GetMy_Text_For_Engine))
      (Widget|SetVisibility _returnvalue_3 "Visible")
      (Class|PlayerController|ClientPlayCameraShake _returnvalue_2 "/Game/Content_AGV/Blueprints/ScreenShakeAGV.ScreenShakeAGV_C" 1.0 "CameraLocal" "0, 0, 0")
      (Input|DisableInput _returnvalue _returnvalue_2)
      (Rendering|ToggleVisibility (Variables|Default|GetTextRender) false)
      (Utilities|FlowControl|Delay 3.0)
      (Input|EnableInput _returnvalue (Game|GetPlayerController 0)))))

(event Collision|EventActorEndOverlap
  (params (OtherActor :type Actor%20Object%20Reference))
  (Variables|/Game/Content_AGV/UI/Dialogue_Box_WIDG.Dialogue_Box_WIDG_C|SetMy_Text (stale Collision|EventActorBeginOverlap _returnvalue_3) (Variables|Default|GetMy_Text_For_Engine))
  (Widget|SetVisibility (stale Collision|EventActorBeginOverlap _returnvalue_3) "Hidden")
  (Widget|SetVisibility (Variables|/Game/Content_AGV/UI/Dialogue_Box_WIDG.Dialogue_Box_WIDG_C|GetDialogue_Box_AGV (stale Collision|EventActorBeginOverlap _returnvalue_3)) "Hidden")
  (Utilities|FlowControl|Delay 5.0)
  (Rendering|ToggleVisibility (Variables|Default|GetTextRender) false)
  (Utilities|FlowControl|Delay 3.0)
  (Input|EnableInput (Game|GetPlayerCharacter 0) (Game|GetPlayerController 0)))

(fn ConstructionScript)