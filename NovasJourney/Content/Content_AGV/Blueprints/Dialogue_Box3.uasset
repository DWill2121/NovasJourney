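; Dialogue_Box3 is a one-shot overlap trigger actor for a dialogue moment.
; On the first overlap it plays the ScreenShakeAGV camera shake, creates a Dialogue_Box_WIDG widget and disables player character input for a few seconds.
; The graph never adds the widget to the viewport itself, and the end-overlap event runs only a delay with nothing after it.
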(event Collision|EventActorBeginOverlap
  (params (OtherActor :type Actor%20Object%20Reference))
  (bind _returnvalue (Game|GetPlayerController 0))
  (bind _returnvalue_2 (Game|GetPlayerCharacter 0))
  (Utilities|FlowControl|DoOnce false
    (:Completed
      (Class|PlayerController|ClientPlayCameraShake (Game|GetPlayerController 0) "/Game/Content_AGV/Blueprints/ScreenShakeAGV.ScreenShakeAGV_C" 1.0 "CameraLocal" "0, 0, 0")
      (UserInterface|CreateWidget "/Game/Content_AGV/UI/Dialogue_Box_WIDG.Dialogue_Box_WIDG_C")
      (Input|DisableInput _returnvalue_2 _returnvalue)
      (Utilities|FlowControl|Delay 3.0)
      (Input|EnableInput _returnvalue_2 _returnvalue))))

(event Collision|EventActorEndOverlap
  (params (OtherActor :type Actor%20Object%20Reference))
  (Utilities|FlowControl|Delay 12.0))

(fn ConstructionScript)